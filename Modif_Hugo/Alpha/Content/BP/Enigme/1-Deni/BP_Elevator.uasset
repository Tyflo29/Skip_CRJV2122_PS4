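; BP_Elevator is an elevator that moves when the first-person character enters its trigger box.
; The overlap plays an elevator door bell sound at the mesh's relative location, waits briefly, then saves that location as the start point.
; A timeline then offsets the static mesh from that start point each update, without sweeping.
; The graph contains no return movement.
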(event OnComponentBeginOverlap(Box)
  (params (OverlappedComponent :type Primitive%20Component%20Object%20Reference) (OtherActor :type Actor%20Object%20Reference) (OtherComp :type Primitive%20Component%20Object%20Reference) (OtherBodyIndex :type Integer) (bFromSweep :type Boolean) (SweepResult :type Hit%20Result%20Structure%20%28by%20ref%29))
  (bind _staticmesh (Variables|Default|GetStaticMesh))
  (bind _relativelocation (Variables|/Script/Engine.SceneComponent|GetRelativeLocation _staticmesh))
  (Utilities|Casting|CastToBP_FirstPersonCharacter OtherActor)
  (Audio|PlaySoundatLocation "/Game/Sound/ASCENSEUR_3_Porte_d39ascenseur_avec_cloche_bruitage_gratuit-YTConverter_app.ASCENSEUR_3_Porte_d39ascenseur_avec_cloche_bruitage_gratuit-YTConverter_app" _relativelocation "0, 0, 0" 1.0 1.0 0.0 0 0 0)
  (Utilities|FlowControl|Delay 3.0)
  (Variables|Default|SetStart _relativelocation)
  (bind _newtrack_2 (Timeline|Timeline_0 Play)
    (:Update
      (Transformation|SetRelativeLocation (Variables|Default|GetStaticMesh) (+ _newtrack_2 (Variables|Default|GetStart)) false false))))

(fn ConstructionScript)