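; Signage actor that pairs a configurable gameplay mesh with a sphere using the M_GMP_Signage material.
; The construction script uniformly scales the sphere by ObjectSize and creates a dynamic instance of that material on its first slot.
; It also assigns GameplayMesh to the GameplayObject component.
; The dynamic instance is not stored, and no material parameters are set here.
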(fn ConstructionScript
  (Transformation|SetRelativeScale3D (Variables|Default|GetSphere) (* "1.000000,1.000000,1.000000" (Variables|Default|GetObject_Size)))
  (Rendering|Material|CreateDynamicMaterialInstance (Variables|Default|GetSphere) 0 "/Game/Matérials/Shader/M_GMP_Signage.M_GMP_Signage" "None" :!class /Script/Engine.PrimitiveComponent)
  (Components|StaticMesh|SetStaticMesh (Variables|Default|GetGameplayObject) (Variables|Default|GetGameplayMesh)))