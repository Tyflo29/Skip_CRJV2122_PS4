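; Post-process actor for the "Marchandage" sequence that pulses a screen effect, apparently a blur, alongside a clock sound.
; MarchandageCall with SoundValue 1 plays the sound at the trigger box's relative location, then runs TimelineBlur to drive the PostProcess blend weight.
; A Delay hung off the timeline's Update reverses it after a short hold.
; The construction script applies the exposed box size and initial blend weight; no overlap logic is present.
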(event EventMarchandageCall
  (params (SoundValue :type Integer))
  (if (== SoundValue 1)
    (Utilities|FlowControl|Sequence
      (:then_0
        (Audio|PlaySoundatLocation "/Game/Sound/SFB-horloge-4.SFB-horloge-4" (Variables|/Script/Engine.SceneComponent|GetRelativeLocation (Variables|Default|GetVolumeTrigger)) "0, 0, 0" 1.0 1.0 0.0 0 0 0))
      (:then_1
        (bind _valueblur (Timeline|TimelineBlur Play)
          (:Update
            (Variables|/Script/Engine.PostProcessComponent|SetBlendWeight (Variables|Default|GetPostProcess) _valueblur)
            (Utilities|FlowControl|Delay 2.5)
            (Timeline|TimelineBlur Reverse)))))))

(fn ConstructionScript
  (Components|Box|SetBoxExtent (Variables|Default|GetVolumeTrigger) (Variables|PostProcessSettings|GetVolumeSize) true)
  (Variables|/Script/Engine.PostProcessComponent|SetBlendWeight (Variables|Default|GetPostProcess) (Variables|Default|GetBlend%20Weight)))