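; Elevator double-door actor that opens when it receives a BasicActorsCommunication call and closes when something overlaps Box1.
; Opening hides Porte and, guarded by a one-time Open flag, plays a timeline that slides PorteG and PorteD apart along local X.
; Closing requires Close, waits briefly, then flips the direction multipliers and reverses the timeline.
; Each update adds the scaled track value to the panels' current positions, so movement is cumulative.
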(event OnComponentBeginOverlap(Box1)
  (params (OverlappedComponent :type Primitive%20Component%20Object%20Reference) (OtherActor :type Actor%20Object%20Reference) (OtherComp :type Primitive%20Component%20Object%20Reference) (OtherBodyIndex :type Integer) (bFromSweep :type Boolean) (SweepResult :type Hit%20Result%20Structure%20%28by%20ref%29))
  (bind _porte_g (Variables|Default|GetPorte_G))
  (bind _porte_d (Variables|Default|GetPorte_D))
  (bind _relativelocation (Variables|/Script/Engine.SceneComponent|GetRelativeLocation _porte_g))
  (bind _relativelocation_2 (Variables|/Script/Engine.SceneComponent|GetRelativeLocation _porte_d))
  (if (Variables|Default|GetClose)
    (Variables|Default|SetClose true)
    (Utilities|FlowControl|Delay 0.5)
    (Variables|Default|SetD -0.505)
    (Variables|Default|SetG 0.505)
    (bind _doortrack (Timeline|Timeline_0 Reverse)
      (:Update
        (Utilities|FlowControl|Sequence
          (:then_0
            (Transformation|SetRelativeLocation _porte_g (Math|Vector|MakeVector (+ (.x _relativelocation) (* _doortrack (Variables|Default|GetG))) (.y _relativelocation) (.z _relativelocation)) false false))
          (:then_1
            (Transformation|SetRelativeLocation _porte_d (Math|Vector|MakeVector (+ (* _doortrack (Variables|Default|GetD)) (.x _relativelocation_2)) (.y _relativelocation_2) (.z _relativelocation_2)) false false)))))))

(event EventBasicActorsCommunication
  (params (True? :type Boolean))
  (bind _porte_g (Variables|Default|GetPorte_G))
  (bind _porte_d (Variables|Default|GetPorte_D))
  (bind _relativelocation (Variables|/Script/Engine.SceneComponent|GetRelativeLocation _porte_g))
  (bind _relativelocation_2 (Variables|/Script/Engine.SceneComponent|GetRelativeLocation _porte_d))
  (Development|PrintString "Open2")
  (Development|SetHiddeninGame (Variables|Default|GetPorte) true false)
  (if (Variables|Default|GetOpen)
    (Variables|Default|SetOpen false)
    (Development|PrintString "Open")
    (Variables|Default|SetD 0.5)
    (Variables|Default|SetG -0.5)
    (bind _doortrack (Timeline|Timeline_0 Play)
      (:Update
        (Utilities|FlowControl|Sequence
          (:then_0
            (Transformation|SetRelativeLocation _porte_g (Math|Vector|MakeVector (+ (.x _relativelocation) (* _doortrack (Variables|Default|GetG))) (.y _relativelocation) (.z _relativelocation)) false false))
          (:then_1
            (Transformation|SetRelativeLocation _porte_d (Math|Vector|MakeVector (+ (* _doortrack (Variables|Default|GetD)) (.x _relativelocation_2)) (.y _relativelocation_2) (.z _relativelocation_2)) false false)))))))

(fn ConstructionScript)

(fn BasicActorsCommunication
  (params (True? :type Boolean))
  (return))