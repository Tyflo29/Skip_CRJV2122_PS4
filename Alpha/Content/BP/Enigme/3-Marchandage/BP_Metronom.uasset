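; BP_Metronom is the metronome of the Marchandage puzzle, switching its audio between a slow and a fast metronome sound.
; The MarchandageCall event prints a debug string, then increments SoundBase for a SoundValue of 0 or decrements it for 1.
; The result is stored in NumbersSound, which selects the sound set on the Audio component, with no clamping on the counter.
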(event EventMarchandageCall
  (params (SoundValue :type Integer))
  (Development|PrintString "PuzzleM")
  (switch int SoundValue
    (:0
      (bind _result (Math|Integer|IncrementInt (Variables|Default|GetSoundBase))
        (:%20%20
          (bind _output_get (Variables|Default|SetNumbersSound _result))
          (Audio|Components|Audio|SetSound (Variables|Default|GetAudio) (Utilities|Select :Index _output_get :Option%200 "/Game/Sound/MetromSlow.MetromSlow" :Option%201 "/Game/Sound/MetromFast.MetromFast")))))
    (:1
      (bind _result_2 (Math|Integer|DecrementInt (Variables|Default|GetSoundBase))
        (:%20%20
          (bind _output_get_2 (Variables|Default|SetNumbersSound _result_2))
          (Audio|Components|Audio|SetSound (Variables|Default|GetAudio) (Utilities|Select :Index _output_get_2 :Option%200 "/Game/Sound/MetromSlow.MetromSlow" :Option%201 "/Game/Sound/MetromFast.MetromFast")))))))

(fn ConstructionScript)