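; Clock prop for the Marchandage (bargaining) enigma, with a configurable mesh, material and sound, plus a glowing sphere effect.
; Construction applies those choices, places the point light above the mesh bounds, and starts it dark with a transparent dynamic-material sphere.
; New_Mesh plays a timeline driving light intensity and radius, sphere opacity and scale, with size and radius divided by SphereDivide.
; Broke_Mesh reverses that timeline.
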(event Custom|Broke_Mesh
  (bind _sphere_divide (Variables|Default|GetSphere_Divide))
  (bind (_direction _intensity_light _opacity_sphere _object_size _light_radius) (Timeline|Timeline_0 Reverse)
    (:Update
      (Utilities|FlowControl|Sequence
        (:then_0
          (bind _output_get (Variables|Default|SetPoint_Intensity _intensity_light))
          (Rendering|Components|Light|SetIntensity (Variables|Default|GetPointLight1) _output_get))
        (:then_1
          (bind _output_get_2 (Variables|Default|SetOpacity_Sphere _opacity_sphere))
          (Rendering|Material|SetScalarParameterValue (Variables|Default|GetCurrentMaterial) "Opacity" _output_get_2 :!class /Script/Engine.MaterialInstanceDynamic))
        (:then_2
          (bind _output_get_3 (Variables|Default|SetObject_Size (/ _object_size _sphere_divide)))
          (Transformation|SetRelativeScale3D (Variables|Default|GetSphere1) (* "0.250000,0.250000,0.250000" _output_get_3))
          (Variables|Default|SetObject_Size 0.0))
        (:then_3
          (Rendering|Lighting|SetAttenuationRadius (Variables|Default|GetPointLight1) (/ _light_radius _sphere_divide)))))))

(event Custom|New_Mesh
  (bind _sphere_divide (Variables|Default|GetSphere_Divide))
  (bind (_direction _intensity_light _opacity_sphere _object_size _light_radius) (Timeline|Timeline_0 Play)
    (:Update
      (Utilities|FlowControl|Sequence
        (:then_0
          (bind _output_get (Variables|Default|SetPoint_Intensity _intensity_light))
          (Rendering|Components|Light|SetIntensity (Variables|Default|GetPointLight1) _output_get))
        (:then_1
          (bind _output_get_2 (Variables|Default|SetOpacity_Sphere _opacity_sphere))
          (Rendering|Material|SetScalarParameterValue (Variables|Default|GetCurrentMaterial) "Opacity" _output_get_2 :!class /Script/Engine.MaterialInstanceDynamic))
        (:then_2
          (bind _output_get_3 (Variables|Default|SetObject_Size (/ _object_size _sphere_divide)))
          (Transformation|SetRelativeScale3D (Variables|Default|GetSphere1) (* "0.250000,0.250000,0.250000" _output_get_3))
          (Variables|Default|SetObject_Size 0.0))
        (:then_3
          (Rendering|Lighting|SetAttenuationRadius (Variables|Default|GetPointLight1) (/ _light_radius _sphere_divide)))))))

(fn ConstructionScript
  (bind _mesh1 (Variables|Default|GetMesh1))
  (bind _pointlight1 (Variables|Default|GetPointLight1))
  (Components|StaticMesh|SetStaticMesh _mesh1 (Variables|Default|GetMesh_Choix))
  (Rendering|Material|SetMaterial _mesh1 0 (Variables|Default|GetMaterial_Mesh))
  (Transformation|SetRelativeScale3D (Variables|Default|GetSphere1) (* "1.000000,1.000000,1.000000" (Variables|Default|GetObject_Size)))
  (Transformation|SetRelativeLocation _pointlight1 (+ (Math|Vector|MakeVector 0.0 0.0 (Variables|Default|GetHeight_Sphere)) (Math|Vector|MakeVector 0.0 0.0 (.z (.Max (Components|StaticMesh|GetLocalBounds (Variables|Default|GetMesh1)))))) false false)
  (Rendering|Lighting|SetAttenuationRadius _pointlight1 0.0)
  (bind _returnvalue (Rendering|Material|CreateDynamicMaterialInstance (Variables|Default|GetSphere1) 0 "/Game/Matérials/Shader/M_GMP_Signage.M_GMP_Signage" "None" :!class /Script/Engine.PrimitiveComponent))
  (bind _output_get (Variables|Default|SetCurrentMaterial _returnvalue))
  (Rendering|Material|SetScalarParameterValue _output_get "Opacity" 0.0 :!class /Script/Engine.MaterialInstanceDynamic)
  (Rendering|Components|Light|SetIntensity _pointlight1 0.0)
  (Audio|Components|Audio|SetSound (Variables|Default|GetAudio) (Variables|Default|GetSound_Horloge)))