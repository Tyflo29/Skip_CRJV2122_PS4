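; Puzzle object actor for the Colere enigma that switches between a new and a broken state.
; New_Mesh swaps the mesh to a cylinder and plays the Green_Sphere_Halo timeline, while Broke_Mesh swaps to a cone and reverses it.
; The timeline drives a halo through point light intensity and radius, sphere scale, and opacity on a dynamic material instance.
; The construction script creates that material and starts the light and sphere opacity at zero.
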(event Custom|Broke_Mesh
  (Development|PrintString "Broke_Actor")
  (Components|StaticMesh|SetStaticMesh (Variables|Default|GetObject) "/Game/StarterContent/Shapes/Shape_Cone.Shape_Cone")
  (bind (_direction _intensity_light _opacity_sphere _object_size _light_radius) (Timeline|Green_Sphere_Halo Reverse)
    (:Update
      (Utilities|FlowControl|Sequence
        (:then_0
          (bind _output_get (Variables|Default|SetPoint_Intensity _intensity_light))
          (Rendering|Components|Light|SetIntensity (Variables|Default|GetPointLight) _output_get))
        (:then_1
          (bind _output_get_2 (Variables|Default|SetOpacity_Sphere _opacity_sphere))
          (Rendering|Material|SetScalarParameterValue (Variables|Default|GetCurrentMaterial) "Opacity" _output_get_2 :!class /Script/Engine.MaterialInstanceDynamic))
        (:then_2
          (bind _output_get_3 (Variables|Default|SetObject_Size _object_size))
          (Transformation|SetRelativeScale3D (Variables|Default|GetSphere) (* "0.250000,0.250000,0.250000" _output_get_3))
          (Variables|Default|SetObject_Size 0.0))
        (:then_3
          (Rendering|Lighting|SetAttenuationRadius (Variables|Default|GetPointLight) _light_radius))))))

(event Custom|New_Mesh
  (Development|PrintString "New_Actor")
  (Components|StaticMesh|SetStaticMesh (Variables|Default|GetObject) "/Game/StarterContent/Shapes/Shape_Cylinder.Shape_Cylinder")
  (bind (_direction _intensity_light _opacity_sphere _object_size _light_radius) (Timeline|Green_Sphere_Halo Play)
    (:Update
      (Utilities|FlowControl|Sequence
        (:then_0
          (bind _output_get (Variables|Default|SetPoint_Intensity _intensity_light))
          (Rendering|Components|Light|SetIntensity (Variables|Default|GetPointLight) _output_get))
        (:then_1
          (bind _output_get_2 (Variables|Default|SetOpacity_Sphere _opacity_sphere))
          (Rendering|Material|SetScalarParameterValue (Variables|Default|GetCurrentMaterial) "Opacity" _output_get_2 :!class /Script/Engine.MaterialInstanceDynamic))
        (:then_2
          (bind _output_get_3 (Variables|Default|SetObject_Size _object_size))
          (Transformation|SetRelativeScale3D (Variables|Default|GetSphere) (* "0.250000,0.250000,0.250000" _output_get_3))
          (Variables|Default|SetObject_Size 0.0))
        (:then_3
          (Rendering|Lighting|SetAttenuationRadius (Variables|Default|GetPointLight) _light_radius))))))

(fn ConstructionScript
  (Transformation|SetRelativeScale3D (Variables|Default|GetSphere) (* "1.000000,1.000000,1.000000" (Variables|Default|GetObject_Size)))
  (Rendering|Lighting|SetAttenuationRadius (Variables|Default|GetPointLight) 0.0)
  (bind _returnvalue (Rendering|Material|CreateDynamicMaterialInstance (Variables|Default|GetSphere) 0 "/Game/Matérials/Shader/M_GMP_Signage.M_GMP_Signage" "None" :!class /Script/Engine.PrimitiveComponent))
  (bind _output_get (Variables|Default|SetCurrentMaterial _returnvalue))
  (Rendering|Material|SetScalarParameterValue _output_get "Opacity" 0.0 :!class /Script/Engine.MaterialInstanceDynamic)
  (Rendering|Components|Light|SetIntensity (Variables|Default|GetPointLight) 0.0))