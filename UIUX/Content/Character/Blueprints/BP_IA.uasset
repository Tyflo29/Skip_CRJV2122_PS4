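; Enemy AI character that wanders, chases the player on sight and forces them to face it once caught.
; Tick moves it to random reachable points until PawnSensing starts a chase, with a throttled sighting sound.
; Reaching the player sets Catch and starts a self-calling delayed loop that interpolates player and control rotation toward the enemy.
; Loop shutdown and the attack montage, fade and level-load chain are present but never run.
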(event OnSeePawn(PawnSensing)
  (params (Pawn :type Pawn%20Object%20Reference))
  (bind _asbp_first_person_character (Utilities|Casting|CastToBP_FirstPersonCharacter (Game|GetPlayerCharacter 0)))
  (if (not (Variables|Default|GetCatch?))
    (Utilities|FlowControl|Sequence
      (:then_0
        (Utilities|FlowControl|Sequence
          (:then_0
            (Variables|Default|SetCan%20See%20Enemy%20? true)
            (Variables|Default|SetIsChasing%20? true)
            (AI|AIMoveTo self "0, 0, 0" _asbp_first_person_character 5.0 false
              (:OnSuccess
                (CallFunction|CatchPlayer))))
          (:then_1
            (Utilities|FlowControl|RetriggerableDelay 0.6)
            (Variables|Default|SetCan%20See%20Enemy%20? false))))
      (:then_1
        (Utilities|FlowControl|Sequence
          (:then_0
            (Utilities|FlowControl|DoOnce false :!label _label
              (:Completed
                (Audio|PlaySoundatLocation 0 (Transformation|GetActorLocation) "0, 0, 0" 1.0 1.0 0.0 0 0 0))))
          (:then_1
            (Utilities|FlowControl|RetriggerableDelay 1.0)
            (goto _label Reset)))))))

(event Custom|CatchPlayer
  (bind _returnvalue (Game|GetPlayerController 0))
  (Variables|Default|SetCatch? true)
  (Variables|Default|SetShouldLoop? true)
  (bind _asbp_first_person_character (Utilities|Casting|CastToBP_FirstPersonCharacter (Game|GetPlayerCharacter 0)))
  (if (Variables|Default|GetShouldLoop?)
    (Utilities|FlowControl|Delay 0.001)
    (Transformation|SetActorRotation _asbp_first_person_character (Math|Interpolation|RInterpTo (Transformation|GetActorRotation _asbp_first_person_character) (Math|Rotator|FindLookatRotation (Transformation|GetActorLocation _asbp_first_person_character) (Transformation|GetActorLocation)) (Utilities|Time|GetWorldDeltaSeconds) 5.0))
    (Pawn|SetControlRotation _returnvalue (Math|Interpolation|RInterpTo (Pawn|GetControlRotation _returnvalue :!class /Script/Engine.Controller) (Math|Rotator|FindLookatRotation (Transformation|GetActorLocation _asbp_first_person_character) (Transformation|GetActorLocation)) (Utilities|Time|GetWorldDeltaSeconds) 5.0))
    (CallFunction|RotationLoop)
    (Utilities|FlowControl|DoOnce false
      (:Completed
        (Utilities|FlowControl|Sequence)))))

(event Custom|RotationLoop
  (bind _returnvalue (Game|GetPlayerController 0))
  (if (Variables|Default|GetShouldLoop?)
    (Utilities|FlowControl|Delay 0.001)
    (Transformation|SetActorRotation (stale Custom|CatchPlayer _asbp_first_person_character) (Math|Interpolation|RInterpTo (Transformation|GetActorRotation (stale Custom|CatchPlayer _asbp_first_person_character)) (Math|Rotator|FindLookatRotation (Transformation|GetActorLocation (stale Custom|CatchPlayer _asbp_first_person_character)) (Transformation|GetActorLocation)) (Utilities|Time|GetWorldDeltaSeconds) 5.0))
    (Pawn|SetControlRotation _returnvalue (Math|Interpolation|RInterpTo (Pawn|GetControlRotation _returnvalue :!class /Script/Engine.Controller) (Math|Rotator|FindLookatRotation (Transformation|GetActorLocation (stale Custom|CatchPlayer _asbp_first_person_character)) (Transformation|GetActorLocation)) (Utilities|Time|GetWorldDeltaSeconds) 5.0))
    (CallFunction|RotationLoop)
    (Utilities|FlowControl|DoOnce false
      (:Completed
        (Utilities|FlowControl|Sequence)))))

(event EventTick
  (params (DeltaSeconds :type Float%20%28single-precision%29))
  (if (not (Variables|Default|GetCatch?))
    (Utilities|FlowControl|Sequence
      (:then_0
        (if (Variables|Default|GetCan%20See%20Enemy%20?)
          (Utilities|FlowControl|Delay 0.4)
          (if (Variables|Default|GetCan%20See%20Enemy%20?)
            _)))
      (:then_1
        (if (not (Variables|Default|GetIsChasing%20?))
          (Utilities|FlowControl|Delay (Math|Random|RandomFloatinRange 2.0 5.0))
          (AI|AIMoveTo self (.RandomLocation (AI|Navigation|GetRandomReachablePointinRadius (Transformation|GetActorLocation) 1.5e+03 0 0)) 0 5.0 false))))))

(fn ConstructionScript)