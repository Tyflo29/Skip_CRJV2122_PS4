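; BP_Dissolve_Sub is an actor whose cube feeds its location and scale to an inverse dissolve material parameter collection.
; The construction script applies the actor's Material variable to the cube.
; Tick runs through a 0.2-second Delay, throttling writes of world location to Position1 and world scale to Bounds in PC_InverseDissolve.
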(event EventBeginPlay)

(event Collision|EventActorBeginOverlap
  (params (OtherActor :type Actor%20Object%20Reference)))

(event EventTick
  (params (DeltaSeconds :type Float%20%28single-precision%29))
  (bind _cube (Variables|Default|GetCube))
  (Utilities|FlowControl|Delay 0.2)
  (Rendering|Material|SetVectorParameterValue "/Game/Matérials/Dissolve/PC_InverseDissolve.PC_InverseDissolve" "Position1" (Math|Conversions|ToLinearColor(Vector) (Transformation|GetWorldLocation _cube)) :!class /Script/Engine.KismetMaterialLibrary)
  (Rendering|Material|SetVectorParameterValue "/Game/Matérials/Dissolve/PC_InverseDissolve.PC_InverseDissolve" "Bounds" (Math|Conversions|ToLinearColor(Vector) (Transformation|GetWorldScale _cube)) :!class /Script/Engine.KismetMaterialLibrary))

(fn ConstructionScript
  (Rendering|Material|SetMaterial (Variables|Default|GetCube) 0 (Variables|Default|GetMaterial)))