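; Clock object for the Marchandage (bargaining) puzzle, switching between In_AIr and Sol (ground) states with a glowing sphere effect.
; Both events toggle gravity and share timelines, played or reversed, that move the mesh vertically and animate sphere scale, opacity and light.
; Sol also notifies BPPPMarchandage and delays the sphere's reversal.
; The construction script sets the chosen mesh and dynamic material; the random-spin NoGravity call is disconnected.
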(event Custom|Sol
  (bind _mesh_object (Variables|Default|GetMesh_Object))
  (bind _sphere_divide (Variables|Default|GetSphere_Divide))
  (bind _relativelocation (Variables|/Script/Engine.SceneComponent|GetRelativeLocation _mesh_object))
  (bind _output_get (Variables|Default|SetNoAir? false))
  (Default|MarchandageCall (Variables|Default|GetBP_PP_Marchandage) 1)
  (Physics|SetEnableGravity (Variables|Default|GetMesh_Object) false)
  (Utilities|FlowControl|Sequence
    (:then_0
      (if _output_get
        (bind (_direction _intensity_light _opacity_sphere _object_size _light_radius) (Timeline|TimelineSphere Play)
          (:Update
            (Utilities|FlowControl|Sequence
              (:then_0
                (bind _output_get_2 (Variables|Default|SetPoint_Intensity _intensity_light))
                (Rendering|Components|Light|SetIntensity (Variables|Default|GetPointLight1) _output_get_2))
              (:then_1
                (bind _output_get_3 (Variables|Default|SetOpacity_Sphere _opacity_sphere))
                (Rendering|Material|SetScalarParameterValue (Variables|Default|GetCurrentMaterial) "Opacity" _output_get_3 :!class /Script/Engine.MaterialInstanceDynamic))
              (:then_2
                (bind _output_get_4 (Variables|Default|SetObject_Size (/ _object_size _sphere_divide)))
                (Transformation|SetRelativeScale3D (Variables|Default|GetSphere) (* "0.250000,0.250000,0.250000" _output_get_4))
                (Variables|Default|SetObject_Size 0.0))
              (:then_3
                (Rendering|Lighting|SetAttenuationRadius (Variables|Default|GetPointLight1) (/ _light_radius _sphere_divide))))))
        (else
          (Utilities|FlowControl|Delay 0.7)
          (Timeline|TimelineSphere Reverse))))
    (:then_1
      (if _output_get
        (Variables|Default|SetAirValue -1.0)
        (bind _valuevector (Timeline|TimeAir Play)
          (:Update
            (Transformation|SetRelativeLocation _mesh_object (Math|Vector|MakeVector (.x _relativelocation) (.y _relativelocation) (+ (.z _relativelocation) (* _valuevector (Variables|Default|GetAirValue)))) true false)))
        (else
          (Variables|Default|SetAirValue 1.0)
          (Default|MarchandageCall (Variables|Default|GetBP_PP_Marchandage))
          (Timeline|TimeAir Reverse))))))

(event Custom|In_AIr
  (bind _mesh_object (Variables|Default|GetMesh_Object))
  (bind _mesh_object_2 (Variables|Default|GetMesh_Object))
  (bind _sphere_divide (Variables|Default|GetSphere_Divide))
  (bind _relativelocation (Variables|/Script/Engine.SceneComponent|GetRelativeLocation _mesh_object_2))
  (Variables|Default|SetNoAir? true)
  (Transformation|SetRelativeRotation _mesh_object "0, 0, 0" false false)
  (Physics|SetEnableGravity _mesh_object true)
  (Utilities|FlowControl|Sequence
    (:then_0
      (if (stale Custom|Sol _output_get)
        (bind (_direction _intensity_light _opacity_sphere _object_size _light_radius) (Timeline|TimelineSphere Play)
          (:Update
            (Utilities|FlowControl|Sequence
              (:then_0
                (bind _output_get (Variables|Default|SetPoint_Intensity _intensity_light))
                (Rendering|Components|Light|SetIntensity (Variables|Default|GetPointLight1) _output_get))
              (:then_1
                (bind _output_get_2 (Variables|Default|SetOpacity_Sphere _opacity_sphere))
                (Rendering|Material|SetScalarParameterValue (Variables|Default|GetCurrentMaterial) "Opacity" _output_get_2 :!class /Script/Engine.MaterialInstanceDynamic))
              (:then_2
                (bind _output_get_3 (Variables|Default|SetObject_Size (/ _object_size _sphere_divide)))
                (Transformation|SetRelativeScale3D (Variables|Default|GetSphere) (* "0.250000,0.250000,0.250000" _output_get_3))
                (Variables|Default|SetObject_Size 0.0))
              (:then_3
                (Rendering|Lighting|SetAttenuationRadius (Variables|Default|GetPointLight1) (/ _light_radius _sphere_divide))))))
        (else
          (Utilities|FlowControl|Delay 0.7)
          (Timeline|TimelineSphere Reverse))))
    (:then_1
      (if (stale Custom|Sol _output_get)
        (Variables|Default|SetAirValue -1.0)
        (bind _valuevector (Timeline|TimeAir Play)
          (:Update
            (Transformation|SetRelativeLocation _mesh_object_2 (Math|Vector|MakeVector (.x _relativelocation) (.y _relativelocation) (+ (.z _relativelocation) (* _valuevector (Variables|Default|GetAirValue)))) true false)))
        (else
          (Variables|Default|SetAirValue 1.0)
          (Default|MarchandageCall (Variables|Default|GetBP_PP_Marchandage))
          (Timeline|TimeAir Reverse))))))

(event Custom|NoGravity
  (Class|PrimitiveComponent|SetPhysicsAngularVelocityinDegrees (Variables|Default|GetMesh_Object) (* (Math|Vector|MakeVector (* (Math|Random|RandomIntegerinRange -1 1) (Math|Random|RandomFloatinRange 1.0 5.0)) (* (Math|Random|RandomIntegerinRange -1 1) (Math|Random|RandomFloatinRange 1.0 5.0)) (* (Math|Random|RandomIntegerinRange -1 1) (Math|Random|RandomFloatinRange 1.0 5.0))) 2e+05) false "None"))

(event Custom|Gravity
  (Class|PrimitiveComponent|SetPhysicsAngularVelocityinDegrees (Variables|Default|GetMesh_Object) "0, 0, 0" false "None"))

(event EventBeginPlay)

(fn ConstructionScript
  (bind _pointlight1 (Variables|Default|GetPointLight1))
  (Components|StaticMesh|SetStaticMesh (Variables|Default|GetMesh_Object) (Variables|Default|GetMesh_Choix))
  (Transformation|SetWorldLocationAndRotation (Variables|Default|GetMesh_Object) (+ (Variables|/Script/Engine.SceneComponent|GetRelativeLocation (Variables|Default|GetDefaultSceneRoot)) "0, 0,128.000000") "0, 0, 0" false false)
  (Transformation|SetRelativeScale3D (Variables|Default|GetSphere) (* "1.000000,1.000000,1.000000" (Variables|Default|GetObject_Size)))
  (Transformation|SetRelativeLocation _pointlight1 (+ (Math|Vector|MakeVector 0.0 0.0 (Variables|Default|GetHeight_Sphere)) (Math|Vector|MakeVector 0.0 0.0 (.z (.Max (Components|StaticMesh|GetLocalBounds (Variables|Default|GetMesh_Object)))))) false false)
  (Rendering|Lighting|SetAttenuationRadius _pointlight1 0.0)
  (bind _returnvalue (Rendering|Material|CreateDynamicMaterialInstance (Variables|Default|GetSphere) 0 "/Game/Matérials/Shader/M_GMP_Signage.M_GMP_Signage" "None" :!class /Script/Engine.PrimitiveComponent))
  (bind _output_get (Variables|Default|SetCurrentMaterial _returnvalue))
  (Rendering|Material|SetScalarParameterValue _output_get "Opacity" 0.0 :!class /Script/Engine.MaterialInstanceDynamic)
  (Rendering|Components|Light|SetIntensity _pointlight1 0.0))