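; BP_Affiche_ID-0 is a poster actor in the first enigma (Deni) that can be shown or hidden.
; Reveal makes the front (Devant) and back (Derrière) components and their children visible and sets IsRevealed.
; Hide acts only when IsRevealed is set, hiding both sides, clearing the flag and printing a debug string.
; Nothing inside the Blueprint calls either function, as BeginPlay and the construction script are empty.
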(event EventBeginPlay)

(fn ConstructionScript)

(fn Hide
  (if (Variables|Default|GetisRevealed)
    (Rendering|SetVisibility (Variables|Default|GetDevant) false true)
    (Variables|Default|SetisRevealed false)
    (Development|PrintString "Hello")))

(fn Reveal
  (Rendering|SetVisibility (Variables|Default|GetDevant) true true)
  (Variables|Default|SetisRevealed true))