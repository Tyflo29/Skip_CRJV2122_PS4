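; One-shot trigger that signals the DeniElevator when the player carries a grief-stage flag: Deni1, Colère, Marchandage1 or Depression1.
; On any actor overlap, it reads these flags from player 0's BP_FirstPersonCharacter and, if any is set, passes all four through DeniCallMessage.
; It then destroys itself and clears every flag on the character except Depression1, which stays set.
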(event Collision|EventActorBeginOverlap
  (params (OtherActor :type Actor%20Object%20Reference))
  (bind _asbp_first_person_character (Utilities|Casting|CastToBP_FirstPersonCharacter (Game|GetPlayerCharacter 0)))
  (if (Math|Boolean|ORBoolean (Variables|/Game/Character/Blueprints/BP_FirstPersonCharacter.BP_FirstPersonCharacter_C|GetDeni_1 _asbp_first_person_character) (Variables|/Game/Character/Blueprints/BP_FirstPersonCharacter.BP_FirstPersonCharacter_C|GetColère _asbp_first_person_character) (Variables|/Game/Character/Blueprints/BP_FirstPersonCharacter.BP_FirstPersonCharacter_C|GetMarchandage%201 _asbp_first_person_character) (Variables|/Game/Character/Blueprints/BP_FirstPersonCharacter.BP_FirstPersonCharacter_C|GetDepression%201 _asbp_first_person_character))
    (Class|BIDefault|DeniCall(Message) (Variables|Default|GetdeniElevator) (Variables|/Game/Character/Blueprints/BP_FirstPersonCharacter.BP_FirstPersonCharacter_C|GetDeni_1 _asbp_first_person_character) (Variables|/Game/Character/Blueprints/BP_FirstPersonCharacter.BP_FirstPersonCharacter_C|GetColère _asbp_first_person_character) (Variables|/Game/Character/Blueprints/BP_FirstPersonCharacter.BP_FirstPersonCharacter_C|GetMarchandage%201 _asbp_first_person_character) (Variables|/Game/Character/Blueprints/BP_FirstPersonCharacter.BP_FirstPersonCharacter_C|GetDepression%201 _asbp_first_person_character))
    (Actor|DestroyActor)
    (Variables|/Game/Character/Blueprints/BP_FirstPersonCharacter.BP_FirstPersonCharacter_C|SetDeni_1 _asbp_first_person_character false)
    (Variables|/Game/Character/Blueprints/BP_FirstPersonCharacter.BP_FirstPersonCharacter_C|SetColère _asbp_first_person_character false)
    (Variables|/Game/Character/Blueprints/BP_FirstPersonCharacter.BP_FirstPersonCharacter_C|SetMarchandage%201 _asbp_first_person_character false)))

(fn ConstructionScript)

(fn BasicActorsCommunication
  (params (True? :type Boolean)))