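; BP_Depression is an actor in the Depression enigma that shows a selectable mesh with a revealable glowing sphere and point light.
; The construction script sets the mesh, places the light above its bounds, zeroes the light and gives the sphere a dynamic material at zero opacity.
; Reveal_Mesh, gated by IsRevealed, plays a timeline driving light intensity, radius and sphere scale; Hide_Mesh re-arms it and reverses the timeline.
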(event Custom|Reveal_Mesh
  (bind _sphere_divide (Variables|Default|GetSphere_Divide))
  (if (Variables|Default|GetisRevealed)
    (Variables|Default|SetisRevealed false)
    (Development|PrintString "PLOT")
    (bind (_direction _intensity_light _opacity_sphere _object_size _light_radius) (Timeline|Timeline_Sphere Play)
      (:Update
        (Utilities|FlowControl|Sequence
          (:then_0
            (bind _output_get (Variables|Default|SetPoint_Intensity _intensity_light))
            (Rendering|Components|Light|SetIntensity (Variables|Default|GetPointLight) _output_get))
          (:then_1
            (Variables|Default|SetOpacity_Sphere _opacity_sphere))
          (:then_2
            (bind _output_get_2 (Variables|Default|SetObject_Size (/ _object_size _sphere_divide)))
            (Transformation|SetRelativeScale3D (Variables|Default|GetSphere) (* "0.250000,0.250000,0.250000" _output_get_2))
            (Variables|Default|SetObject_Size 0.0))
          (:then_3
            (Rendering|Lighting|SetAttenuationRadius (Variables|Default|GetPointLight) (/ _light_radius _sphere_divide))))))))

(event Custom|Hide_Mesh
  (bind _sphere_divide (Variables|Default|GetSphere_Divide))
  (Variables|Default|SetisRevealed true)
  (bind (_direction _intensity_light _opacity_sphere _object_size _light_radius) (Timeline|Timeline_Sphere Reverse)
    (:Update
      (Utilities|FlowControl|Sequence
        (:then_0
          (bind _output_get (Variables|Default|SetPoint_Intensity _intensity_light))
          (Rendering|Components|Light|SetIntensity (Variables|Default|GetPointLight) _output_get))
        (:then_1
          (Variables|Default|SetOpacity_Sphere _opacity_sphere))
        (:then_2
          (bind _output_get_2 (Variables|Default|SetObject_Size (/ _object_size _sphere_divide)))
          (Transformation|SetRelativeScale3D (Variables|Default|GetSphere) (* "0.250000,0.250000,0.250000" _output_get_2))
          (Variables|Default|SetObject_Size 0.0))
        (:then_3
          (Rendering|Lighting|SetAttenuationRadius (Variables|Default|GetPointLight) (/ _light_radius _sphere_divide)))))))

(event EventBeginPlay
  (Variables|Default|SetCurrentLocation (Transformation|GetWorldLocation (Variables|Default|GetMesh))))

(fn ConstructionScript
  (Components|StaticMesh|SetStaticMesh (Variables|Default|GetMesh) (Variables|Default|GetMesh_Choix))
  (Transformation|SetRelativeScale3D (Variables|Default|GetSphere) (* "1.000000,1.000000,1.000000" (Variables|Default|GetObject_Size)))
  (Transformation|SetRelativeLocation (Variables|Default|GetPointLight) (+ (Math|Vector|MakeVector 0.0 0.0 (Variables|Default|GetHeight_Sphere)) (Math|Vector|MakeVector 0.0 0.0 (.z (.Max (Components|StaticMesh|GetLocalBounds (Variables|Default|GetMesh)))))) false false)
  (Rendering|Lighting|SetAttenuationRadius (Variables|Default|GetPointLight) 0.0)
  (bind _returnvalue (Rendering|Material|CreateDynamicMaterialInstance (Variables|Default|GetSphere) 0 "/Game/Matérials/Shader/M_GMP_Signage.M_GMP_Signage" "None" :!class /Script/Engine.PrimitiveComponent))
  (bind _output_get (LocalVariables|SetCurrentMaterial _returnvalue))
  (Rendering|Material|SetScalarParameterValue _output_get "Opacity" 0.0 :!class /Script/Engine.MaterialInstanceDynamic)
  (Rendering|Components|Light|SetIntensity (Variables|Default|GetPointLight) 0.0))