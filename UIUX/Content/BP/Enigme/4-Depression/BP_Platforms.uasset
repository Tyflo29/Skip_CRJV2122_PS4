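; BP_Platforms is a falling platform for the Depression enigma that drops and then resets along with the player.
; BeginPlay caches the mesh's world transform.
; FallPlatforms enables gravity with a custom-plane constraint, waits three seconds, then disables gravity and applies the cached transform as a relative one.
; It also teleports the player character to the ResetDep actor and prints the mesh name when triggered.
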(event Custom|FallPlatforms
  (bind _platformmesh (Variables|Default|GetPlatformMesh))
  (bind _platformmesh_2 (Variables|Default|GetPlatformMesh))
  (bind _reset_dep (Variables|Default|GetReset%20Dep))
  (Development|PrintString (Utilities|GetDisplayName _platformmesh_2))
  (Class|PrimitiveComponent|SetConstraintMode _platformmesh_2 "CustomPlane")
  (Physics|SetEnableGravity _platformmesh_2 true)
  (Utilities|FlowControl|Delay 3.0)
  (Utilities|FlowControl|Sequence
    (:then_0
      (Physics|SetEnableGravity _platformmesh false)
      (Transformation|SetRelativeLocationAndRotation _platformmesh (stale EventBeginPlay _output_get) (stale EventBeginPlay _output_get_2) false false)
      (Class|PrimitiveComponent|SetConstraintMode _platformmesh "Default"))
    (:then_1
      (Transformation|SetActorLocationAndRotation (Game|GetPlayerCharacter 0) (Transformation|GetActorLocation _reset_dep) (Transformation|GetActorRotation _reset_dep) false true))))

(event EventBeginPlay
  (bind _platformmesh (Variables|Default|GetPlatformMesh))
  (bind _output_get (Variables|Default|SetCurrentLocation (Transformation|GetWorldLocation _platformmesh)))
  (bind _output_get_2 (Variables|Default|SetCurrentRotation (Transformation|GetWorldRotation _platformmesh))))

(fn ConstructionScript)