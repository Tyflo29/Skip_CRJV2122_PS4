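; Portal manager that drives the see-through views of a linked pair of portals, Portal1 and Portal2.
; Every tick, each portal's PortalCapture is placed and rotated to mirror the player camera's pose relative to the opposite portal.
; The transform uses the rotation delta between the two portals, with a 180-degree yaw flip.
; An actor overlap only prints a debug string and raises Portal1 along Z; no player teleport is implemented.
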(event Collision|EventActorBeginOverlap
  (params (OtherActor :type Actor%20Object%20Reference))
  (bind _portal1 (Variables|Default|GetPortal1))
  (bind _defaultsceneroot (Variables|/Game/BP/Portal/BP_Portal1.BP_Portal1_C|GetDefaultSceneRoot _portal1))
  (Development|PrintString "Hello")
  (Transformation|SetWorldLocation _defaultsceneroot (+ (Transformation|GetWorldLocation _defaultsceneroot) "0, 0,520.000000") false false))

(event EventTick
  (params (DeltaSeconds :type Float%20%28single-precision%29))
  (CallFunction|Portal1Update)
  (CallFunction|Portal2Update))

(fn ConstructionScript)

(fn Portal1Update
  (bind _returnvalue (Game|GetPlayerCameraManager 0))
  (bind _portal2 (Variables|Default|GetPortal2))
  (bind _portal1 (Variables|Default|GetPortal1))
  (bind _defaultsceneroot (Variables|/Game/BP/Portal/BP_Portal2.BP_Portal2_C|GetDefaultSceneRoot _portal2))
  (bind _transformcomponent (Variables|/Script/Engine.PlayerCameraManager|GetTransformComponent _returnvalue))
  (bind _defaultsceneroot_2 (Variables|/Game/BP/Portal/BP_Portal1.BP_Portal1_C|GetDefaultSceneRoot _portal1))
  (bind _returnvalue_2 (Transformation|GetWorldRotation _defaultsceneroot_2))
  (bind _returnvalue_3 (Transformation|GetWorldRotation _defaultsceneroot))
  (bind _returnvalue_4 (- (.yaw _returnvalue_3) 1.8e+02))
  (bind _returnvalue_5 (Math|Rotator|MakeRotator (.roll _returnvalue_3) (.pitch _returnvalue_3) _returnvalue_4))
  (bind _returnvalue_6 (Math|Rotator|Delta(Rotator) _returnvalue_5 _returnvalue_2))
  (Transformation|SetWorldLocationAndRotation (Variables|/Game/BP/Portal/BP_Portal2.BP_Portal2_C|GetPortalCapture (Variables|Default|GetPortal2)) (+ (- (Transformation|GetWorldLocation _defaultsceneroot) (Math|Vector|RotateVector (Transformation|GetWorldLocation _defaultsceneroot_2) _returnvalue_6)) (Math|Vector|RotateVector (Transformation|GetWorldLocation _transformcomponent) _returnvalue_6)) (Math|Rotator|CombineRotators (Transformation|GetWorldRotation _transformcomponent) _returnvalue_6) false false))

(fn Portal2Update
  (bind _returnvalue (Game|GetPlayerCameraManager 0))
  (bind _portal2 (Variables|Default|GetPortal2))
  (bind _portal1 (Variables|Default|GetPortal1))
  (bind _defaultsceneroot (Variables|/Game/BP/Portal/BP_Portal2.BP_Portal2_C|GetDefaultSceneRoot _portal2))
  (bind _transformcomponent (Variables|/Script/Engine.PlayerCameraManager|GetTransformComponent _returnvalue))
  (bind _defaultsceneroot_2 (Variables|/Game/BP/Portal/BP_Portal1.BP_Portal1_C|GetDefaultSceneRoot _portal1))
  (bind _returnvalue_2 (Transformation|GetWorldRotation _defaultsceneroot))
  (bind _returnvalue_3 (Transformation|GetWorldRotation _defaultsceneroot_2))
  (bind _returnvalue_4 (- (.yaw _returnvalue_3) 1.8e+02))
  (bind _returnvalue_5 (Math|Rotator|MakeRotator (.roll _returnvalue_3) (.pitch _returnvalue_3) _returnvalue_4))
  (bind _returnvalue_6 (Math|Rotator|Delta(Rotator) _returnvalue_5 _returnvalue_2))
  (Transformation|SetWorldLocationAndRotation (Variables|/Game/BP/Portal/BP_Portal1.BP_Portal1_C|GetPortalCapture (Variables|Default|GetPortal1)) (+ (- (Transformation|GetWorldLocation _defaultsceneroot_2) (Math|Vector|RotateVector (Transformation|GetWorldLocation _defaultsceneroot) _returnvalue_6)) (Math|Vector|RotateVector (Transformation|GetWorldLocation _transformcomponent) _returnvalue_6)) (Math|Rotator|CombineRotators (Transformation|GetWorldRotation _transformcomponent) _returnvalue_6) false false))