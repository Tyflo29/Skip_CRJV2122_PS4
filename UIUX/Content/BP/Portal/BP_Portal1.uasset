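; BP_Portal1 is a portal actor that switches its surface material and teleports the first-person player to Portal2.
; A delay-throttled Tick reads the character's Physique flag to choose between two portal materials, apparently render-target based.
; Pressing E while Physique is false moves the player to Portal2's box and sets a fixed yaw.
; The box-overlap check is unwired, so teleporting ignores proximity.
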(event EventTick
  (params (DeltaSeconds :type Float%20%28single-precision%29))
  (Utilities|FlowControl|Delay 0.2)
  (bind _asbp_first_person_character (Utilities|Casting|CastToBP_FirstPersonCharacter (Game|GetPlayerCharacter 0)))
  (if (Variables|/Game/Character/Blueprints/BP_FirstPersonCharacter.BP_FirstPersonCharacter_C|GetPhysique? _asbp_first_person_character)
    (Rendering|Material|SetMaterial (Variables|Default|GetPortal) 0 "/Game/BP/Portal/Portal1_RT_Mat.Portal1_RT_Mat")
    (else
      (Rendering|Material|SetMaterial (Variables|Default|GetPortal) 0 "/Game/BP/Portal/Portal2_RT_Mat.Portal2_RT_Mat"))))

(event Input|KeyboardEvents|E
  (params (Key :type Key%20Structure))
  (bind _returnvalue (Game|GetPlayerCharacter 0))
  (:Pressed
    (if (Math|Boolean|NotEqual(Boolean) (Variables|/Game/Character/Blueprints/BP_FirstPersonCharacter.BP_FirstPersonCharacter_C|GetPhysique? (stale EventTick _asbp_first_person_character)) true)
      (Transformation|Teleport _returnvalue (Transformation|GetWorldLocation (Variables|/Game/BP/Portal/BP_Portal2.BP_Portal2_C|GetBox (Variables|Default|GetPortal_2))) "0, 0, 0")
      (bind _asbp_first_person_character (Utilities|Casting|CastToBP_FirstPersonCharacter _returnvalue))
      (Transformation|SetActorRotation _asbp_first_person_character "90.000000, 0, 0"))))

(fn ConstructionScript)