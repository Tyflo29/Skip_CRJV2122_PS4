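; BP_CarCrashSound is a one-shot ambience trigger that stages an off-screen car crash with lights and sound.
; The construction script hides two spotlights; the first overlap of the Box reveals them.
; The Crash audio component then plays after a short delay while MoveComponentTo slides it along its relative X axis, so the sound source travels.
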(event OnComponentBeginOverlap(Box)
  (params (OverlappedComponent :type Primitive%20Component%20Object%20Reference) (OtherActor :type Actor%20Object%20Reference) (OtherComp :type Primitive%20Component%20Object%20Reference) (OtherBodyIndex :type Integer) (bFromSweep :type Boolean) (SweepResult :type Hit%20Result%20Structure%20%28by%20ref%29))
  (Utilities|FlowControl|DoOnce false
    (:Completed
      (Rendering|SetVisibility (Variables|Default|GetSpotLight) true false)
      (Utilities|FlowControl|Sequence
        (:then_0
          (Utilities|FlowControl|Delay 0.2)
          (Audio|Components|Audio|Play (Variables|Default|GetCrash) 0.0))
        (:then_1
          (Components|MoveComponentTo (Variables|Default|GetCrash) "-1200.000000,0.000000, 0" "0, 0, 0" false false 1.5 false))))))

(fn ConstructionScript
  (Rendering|SetVisibility (Variables|Default|GetSpotLight) false false))