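; Menu actor that, judging by its name and path, scatters random props as menu decoration.
; On BeginPlay, four mesh components each pick one of seven props such as bench, bin or television, while the first gets SetStaticMesh with no mesh specified.
; All five then go through ImpulseForce, which despite its name makes a single AddForce call with randomly signed, random-magnitude axes scaled by a large constant.
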(event EventBeginPlay
  (bind _returnvalue (Math|Random|RandomIntegerinRange 0 6))
  (bind _returnvalue_2 (Utilities|Select :Index _returnvalue :Option%200 "/Game/Mesh/Props/Narratifs/Banc.Banc" :Option%201 "/Game/Mesh/Props/Narratifs/Poubelle.Poubelle" :Option%202 "/Game/Mesh/Props_Moyens/Television/Television.Television" :Option%203 "/Game/Zone_De_Test/Meshes/Props_Moyens/Table/Table.Table" :Option%204 "/Game/Mesh/Props_Moyens/Chaise/Chaise.Chaise" :Option%205 "/Game/Zone_De_Test/Meshes/ANTIchambre/Cadre_Contour.Cadre_Contour" :Option%206 "/Game/Mesh/Props/Narratifs/BoucheAIncendie.BoucheAIncendie"))
  (Components|StaticMesh|SetStaticMesh (Variables|Default|GetStaticMesh) 0)
  (Components|StaticMesh|SetStaticMesh (Variables|Default|GetStaticMesh1) _returnvalue_2)
  (Components|StaticMesh|SetStaticMesh (Variables|Default|GetStaticMesh2) _returnvalue_2)
  (Components|StaticMesh|SetStaticMesh (Variables|Default|GetStaticMesh3) _returnvalue_2)
  (Components|StaticMesh|SetStaticMesh (Variables|Default|GetStaticMesh4) _returnvalue_2)
  (CallFunction|ImpulseForce (Variables|Default|GetStaticMesh))
  (CallFunction|ImpulseForce (Variables|Default|GetStaticMesh1))
  (CallFunction|ImpulseForce (Variables|Default|GetStaticMesh4))
  (CallFunction|ImpulseForce (Variables|Default|GetStaticMesh3))
  (CallFunction|ImpulseForce (Variables|Default|GetStaticMesh2)))

(fn ConstructionScript)

(fn ImpulseForce
  (params (Mesh :type Static%20Mesh%20Component%20Object%20Reference))
  (Physics|AddForce Mesh (* (Math|Vector|MakeVector (* (Utilities|Select :Index (Math|Random|RandomIntegerinRange 0 1) :Option%200 -1 :Option%201 1) (Math|Random|RandomFloat)) (* (Utilities|Select :Index (Math|Random|RandomIntegerinRange 0 1) :Option%200 -1 :Option%201 1) (Math|Random|RandomFloat)) (* (Utilities|Select :Index (Math|Random|RandomIntegerinRange 0 1) :Option%200 -1 :Option%201 1) (Math|Random|RandomFloat))) 2e+05) "None" false))