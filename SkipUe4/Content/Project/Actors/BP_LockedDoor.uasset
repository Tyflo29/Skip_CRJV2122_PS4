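; BP_LockedDoor is a door the player can open and close with the Interaction input while carrying a key.
; A box overlap by the FirstPersonCharacter enables input and opens a gate, and leaving reverses both.
; Interaction checks the character's HasKey, playing a locked sound without it.
; With it, a sound plays and a FlipFlop alternately plays or reverses a timeline that lerps the mesh yaw between closed and open angles.
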(event OnComponentBeginOverlap(Box)
  (params (OverlappedComponent :type Primitive%20Component%20Object%20Reference) (OtherActor :type Actor%20Object%20Reference) (OtherComp :type Primitive%20Component%20Object%20Reference) (OtherBodyIndex :type Integer) (bFromSweep :type Boolean) (SweepResult :type Hit%20Result%20Structure%20%28by%20ref%29))
  (bind _asfirst_person_character (Utilities|Casting|CastToFirstPersonCharacter OtherActor))
  (Input|EnableInput (Game|GetPlayerController 0))
  (Utilities|FlowControl|Gate true) ; enters at Open
)

(event OnComponentEndOverlap(Box)
  (params (OverlappedComponent :type Primitive%20Component%20Object%20Reference) (OtherActor :type Actor%20Object%20Reference) (OtherComp :type Primitive%20Component%20Object%20Reference) (OtherBodyIndex :type Integer))
  (Utilities|Casting|CastToFirstPersonCharacter OtherActor)
  (Input|DisableInput (Game|GetPlayerController 0))
  (Utilities|FlowControl|Gate true) ; enters at Close
)

(event Input|ActionEvents|InputActionInteraction
  (params (Key :type Key%20Structure :default "None"))
  (:Pressed
    (if (Variables|/Game/FirstPersonBP/Blueprints/FirstPersonCharacter_Auto3.FirstPersonCharacter_C|GetHasKey? (stale OnComponentBeginOverlap(Box) _asfirst_person_character))
      (Utilities|FlowControl|Gate true
        (:Exit
          (Audio|PlaySoundatLocation "/Game/Project/Sound/DoorOpening2.DoorOpening2" (Transformation|GetActorLocation) "0, 0, 0" 1.0 1.0 0.0 0 0 0)
          (Utilities|FlowControl|FlipFlop
            (:A
              (bind _doortrack (Timeline|Open/CloseDoor Play)
                (:Update
                  (Transformation|SetRelativeRotation (Variables|Default|GetStaticMesh) (Math|Rotator|MakeRotator 0.0 0.0 (Math|Float|Lerp (Variables|Default|GetClosed%20Angle) (Variables|Default|GetOpen%20Angle) _doortrack)) false false))))
            (:B
              (Timeline|Open/CloseDoor Reverse)))))
      (else
        (Audio|PlaySoundatLocation "/Game/Project/Sound/LockedPlayerSoundEffect__1_.LockedPlayerSoundEffect__1_" (Transformation|GetActorLocation) "0, 0, 0" 1.0 1.0 0.0 0 0 0)))))

(fn ConstructionScript)