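; BP_Walls is a triggered set piece that moves three walls and animates a plane on the FirstPersonCharacter.
; The first box destroys itself on player overlap, then timelines offset each wall from its starting relative location.
; Shortly after, a dynamic M_Plane instance on the character's Plane animates R_Fade and T_Fade together, then C_Fade once T finishes.
; The second box calls PlaneD on the character and destroys the actor.
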(event OnComponentBeginOverlap(Box)
  (params (OverlappedComponent :type Primitive%20Component%20Object%20Reference) (OtherActor :type Actor%20Object%20Reference) (OtherComp :type Primitive%20Component%20Object%20Reference) (OtherBodyIndex :type Integer) (bFromSweep :type Boolean) (SweepResult :type Hit%20Result%20Structure%20%28by%20ref%29))
  (bind _asfirst_person_character (Utilities|Casting|CastToFirstPersonCharacter OtherActor))
  (Utilities|FlowControl|Sequence
    (:then_0
      (Components|DestroyComponent (Variables|Default|GetBox))
      (Utilities|FlowControl|Sequence
        (:then_0
          (Variables|Default|SetLocation (Variables|/Script/Engine.SceneComponent|GetRelativeLocation (Variables|Default|GetWall1)))
          (bind _newtrack_2 (Timeline|Wall1Moov Play)
            (:Update
              (Transformation|SetRelativeLocation (Variables|Default|GetWall1) (+ _newtrack_2 (Variables|Default|GetLocation)) false false))))
        (:then_1
          (Variables|Default|SetLocation2 (Variables|/Script/Engine.SceneComponent|GetRelativeLocation (Variables|Default|GetWall2)))
          (bind _newtrack_2_2 (Timeline|Timeline_0 Play)
            (:Update
              (Transformation|SetRelativeLocation (Variables|Default|GetWall2) (+ _newtrack_2_2 (Variables|Default|GetLocation2)) false false))))
        (:then_2
          (Variables|Default|Setlocation3 (Variables|/Script/Engine.SceneComponent|GetRelativeLocation (Variables|Default|GetWall3)))
          (bind _newtrack_0 (Timeline|Timeline_1 Play)
            (:Update
              (Transformation|SetRelativeLocation (Variables|Default|GetWall3) (+ _newtrack_0 (Variables|Default|Getlocation3)) false false))))))
    (:then_1
      (Utilities|FlowControl|Delay 0.1)
      (bind _returnvalue (Rendering|Material|CreateDynamicMaterialInstance (Variables|/Game/FirstPersonBP/Blueprints/FirstPersonCharacter_Auto3.FirstPersonCharacter_C|GetPlane _asfirst_person_character) 0 "/Game/Project/Materials/M_Plane.M_Plane" "None" :!class /Script/Engine.PrimitiveComponent))
      (Utilities|FlowControl|Sequence
        (:then_0
          (bind _newtrack_0_2 (Timeline|Timeline_2 PlayFromStart)
            (:Update
              (Rendering|Material|SetScalarParameterValue _returnvalue "R_Fade" _newtrack_0_2 :!class /Script/Engine.MaterialInstanceDynamic))))
        (:then_1
          (bind _newtrack_0_3 (Timeline|Timeline_3 PlayFromStart)
            (:Update
              (Rendering|Material|SetScalarParameterValue _returnvalue "T_Fade" _newtrack_0_3 :!class /Script/Engine.MaterialInstanceDynamic))
            (:Finished
              (bind _newtrack_0_4 (Timeline|Timeline_4 Play)
                (:Update
                  (Rendering|Material|SetScalarParameterValue _returnvalue "C_Fade" _newtrack_0_4 :!class /Script/Engine.MaterialInstanceDynamic))))))))))

(event OnComponentBeginOverlap(Box1)
  (params (OverlappedComponent :type Primitive%20Component%20Object%20Reference) (OtherActor :type Actor%20Object%20Reference) (OtherComp :type Primitive%20Component%20Object%20Reference) (OtherBodyIndex :type Integer) (bFromSweep :type Boolean) (SweepResult :type Hit%20Result%20Structure%20%28by%20ref%29))
  (bind _asfirst_person_character (Utilities|Casting|CastToFirstPersonCharacter OtherActor))
  (Default|PlaneD _asfirst_person_character)
  (Actor|DestroyActor))

(fn ConstructionScript)

(fn NewFunction0
  (params (curve :type Curve%20Float%20Object%20Reference)))