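; BP_Flo_2 is a test-zone trigger that sets five static meshes moving with physics forces when its Box is overlapped.
; The overlap spins and pushes the meshes in different directions, then destroys the Box component.
; StaticMesh also enters LaunchSM1, a self-calling event that zeroes its velocity and reapplies the force with reversed sign after each delay, producing an endless back-and-forth.
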(event OnComponentBeginOverlap(Box)
  (params (OverlappedComponent :type Primitive%20Component%20Object%20Reference) (OtherActor :type Actor%20Object%20Reference) (OtherComp :type Primitive%20Component%20Object%20Reference) (OtherBodyIndex :type Integer) (bFromSweep :type Boolean) (SweepResult :type Hit%20Result%20Structure%20%28by%20ref%29))
  (bind _staticmesh (Variables|Default|GetStaticMesh))
  (Utilities|FlowControl|Sequence
    (:then_0
      (Class|PrimitiveComponent|AddAngularImpulseinDegrees _staticmesh "100000.000000,0.000000,10000.000000" "None" false)
      (CallFunction|LaunchSM1 _staticmesh "100000.000000, 0, 0" 1))
    (:then_1
      (Physics|AddForce (Variables|Default|GetStaticMesh1) "0.000000,200000.000000,1500.000000" "None" false)
      (Class|PrimitiveComponent|AddAngularImpulseinDegrees (Variables|Default|GetStaticMesh1) "2000000.000000,0.000000,2000000.000000" "None" false)
      (Components|DestroyComponent (Variables|Default|GetBox)))
    (:then_2
      (Physics|AddForce (Variables|Default|GetStaticMesh2) "0.000000,0.000000,100000.000000" "None" false)
      (Class|PrimitiveComponent|AddAngularImpulseinDegrees (Variables|Default|GetStaticMesh2) "1000000.000000,0.000000,1000000.000000" "None" false))))

(event Custom|LaunchSM1
  (params (Target :type Primitive%20Component%20Object%20Reference) (Direction :type Vector) (Sign :type Integer))
  (Physics|SetPhysicsLinearVelocity Target "0, 0, 0" false "None")
  (Physics|AddForce Target (* Direction Sign) "None" false)
  (Utilities|FlowControl|Delay 12.0)
  (CallFunction|LaunchSM1 Target Direction (* Sign -1)))

(fn ConstructionScript)