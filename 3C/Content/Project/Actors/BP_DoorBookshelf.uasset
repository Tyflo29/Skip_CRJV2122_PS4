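; Bookshelf door actor that swings open, with a special book that tilts as its trigger animation.
; Open/ClosedDoor alternates through a FlipFlop, with a DoOnce blocking re-triggers until the running timeline finishes.
; The open branch plays OpenTrack, rolling SpecialBook and yawing the root between closed and open angles.
; The close branch reverses a separate Timeline_0 on DoorBook with both yaw endpoints zero, leaving book and root unrestored.
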(event Custom|Open/ClosedDoor
  (Utilities|FlowControl|DoOnce false :!label _label
    (:Completed
      (Utilities|FlowControl|FlipFlop
        (:A
          (bind (_direction _booktrack _doorbooktrack) (Timeline|OpenTrack PlayFromStart)
            (:Update
              (Transformation|SetRelativeRotation (Variables|Default|GetSpecialBook) (Math|Rotator|MakeRotator (Math|Float|Lerp (Variables|Default|GetBookIn) (Variables|Default|GetBookOut) _booktrack) 0.0 0.0) false false)
              (Transformation|SetWorldRotation (Variables|Default|GetDefaultSceneRoot) (Math|Rotator|MakeRotator 0.0 0.0 (Math|Float|Lerp (Variables|Default|GetDoorClosed) (Variables|Default|GetDoorOpen) _doorbooktrack)) false false))
            (:Finished
              (goto _label Reset))))
        (:B
          (bind _doortrack (Timeline|Timeline_0 ReverseFromEnd)
            (:Update
              (Transformation|SetRelativeRotation (Variables|Default|GetDoorBook) (Math|Rotator|MakeRotator 0.0 0.0 (Math|Float|Lerp 0.0 0.0 _doortrack)) false false))
            (:Finished
              (goto _label Reset))))))))

(fn ConstructionScript)