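; BP_Bookshelf is a one-shot scripted event in which a book is shoved by physics when the first-person player enters a trigger box.
; On overlap, the Book starts simulating, receives a single strong push along world +Y, and the Box is destroyed to prevent retriggering.
; After a short delay, a BP_InspectableItemParent actor spawns at the Book's location and rotation with unit scale, and the Book component is destroyed.
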(event OnComponentBeginOverlap(Box)
  (params (OverlappedComponent :type Primitive%20Component%20Object%20Reference) (OtherActor :type Actor%20Object%20Reference) (OtherComp :type Primitive%20Component%20Object%20Reference) (OtherBodyIndex :type Integer) (bFromSweep :type Boolean) (SweepResult :type Hit%20Result%20Structure%20%28by%20ref%29))
  (bind _book (Variables|Default|GetBook))
  (bind _book_2 (Variables|Default|GetBook))
  (bind _returnvalue (Transformation|GetWorldTransform _book_2))
  (bind (_location _rotation) (Math|Transform|BreakTransform _returnvalue))
  (Utilities|Casting|CastToFirstPersonCharacter OtherActor)
  (Physics|SetSimulatePhysics _book true)
  (Physics|AddForce _book "0.000000,400000.000000,0.000000" "None" false)
  (Components|DestroyComponent (Variables|Default|GetBox))
  (Utilities|FlowControl|Delay 3.0)
  (Game|SpawnActorfromClass "/Game/Project/Actors/BP_InspectableItemParent.BP_InspectableItemParent_C" (Math|Transform|MakeTransform _location _rotation) "Undefined" 0 0)
  (Components|DestroyComponent (Variables|Default|GetBook)))

(fn ConstructionScript)